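; BP_LightActor is a light actor that flashes its PointLight a set number of times after play begins.
; BeginPlay starts a delayed looping timer whose interval is the reciprocal of Speed, written as Speed over its square.
; Each IsOnLight call sets visibility from OnLight, flips that flag and increments Count.
; The timer is cleared once Count reaches twice CountFlash, as each flash takes two toggles.
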(event EventBeginPlay
  (bind _speed (Variables|Light|GetSpeed))
  (Utilities|IsValid (Variables|Default|GetPointLight)
    (:Is%20Valid
      (Utilities|Time|SetTimerbyFunctionName 0 "IsOnLight" (/ _speed (Math|Float|Square _speed)) true (Variables|Light|GetStartDelay)))))

(event Collision|EventActorBeginOverlap
  (params (OtherActor :type Actor%20Object%20Reference)))

(event EventTick
  (params (DeltaSeconds :type Float%20%28single-precision%29)))

(fn ConstructionScript)

(fn IsonLight
  (Rendering|SetVisibility (Variables|Default|GetPointLight) (Variables|Default|GetOnLight) false)
  (Variables|Default|SetOnLight (not (Variables|Default|GetOnLight)))
  (bind _result (Math|Float|IncrementFloat (Variables|Default|GetCount))
    (:%20%20
      (bind _output_get (Variables|Default|SetCount _result))
      (if (>= _output_get (* (Variables|Light|GetCountFlash) 2.0))
        (Utilities|Time|ClearTimerbyFunctionName 0 "IsOnLight")))))